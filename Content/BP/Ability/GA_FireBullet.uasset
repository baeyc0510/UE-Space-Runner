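; Gameplay ability that fires a single bullet from the player character, then ends immediately.
; Activation caches the avatar as BP_PlayerCharacter and fires only if the ability commit succeeds.
; Fire pulls BP_Bullet from a pool at the fire point, initializing it with Arrow run-state stats, with speed and range scaled by base values.
; Spread firing is marked as a TODO.
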(event `self.K2_ActivateAbility`
  (`parent.K2_ActivateAbility`)
  (`|ExecutionSequence`
    (:`then_0`
      (`/Engine/EditorBlueprintResources/StandardMacros.IsValid` (`self.PlayerCharacter`)
        (:`Is Not Valid`
          (bind _asbp_player_character (cast `/Game/BP/Characters/Player/BP_PlayerCharacter` (`self.GetAvatarActorFromActorInfo`)))
          (set `self.PlayerCharacter` _asbp_player_character))))
    (:`then_1`
      (`/Engine/EditorBlueprintResources/StandardMacros.IsValid` (`self.PlayerCharacter`)
        (:`Is Valid`
          (bind _returnvalue (`self.K2_CommitAbility`))
          (if _returnvalue
            (`self.Fire`)
            (`self.K2_EndAbility`)
            (else
              (`self.K2_EndAbility`))))
        (:`Is Not Valid`
          (`self.K2_EndAbility`))))))

(event `self.K2_OnEndAbility`
  (params (bWasCancelled :type Boolean))
  (`parent.K2_OnEndAbility` bWasCancelled))

(fn `Fire`
  (bind _returnvalue (`ObjectPoolBlueprintLibrary.SpawnFromPool` "/Game/BP/Projectile/BP_Bullet.BP_Bullet_C" (`KismetMathLibrary.MakeTransform` (`/Game/BP/Characters/Player/BP_PlayerCharacter.GetFirePoint` (`self.PlayerCharacter`)) (`Actor.K2_GetActorRotation` (`self.PlayerCharacter`))) "AlwaysSpawn"))
  (`/Game/BP/Projectile/BP_Bullet.InitBullet` _returnvalue (`self.GetAvatarActorFromActorInfo`) (`RogueliteBlueprintLibrary.GetRunStateValue` (struct :`TagName` "Stat.Ability.Arrow.Power")) (* (`RogueliteBlueprintLibrary.GetRunStateValue` (struct :`TagName` "Stat.Ability.Arrow.Speed") 0.1) (`self.BaseBulletSpeed`)) (* (`RogueliteBlueprintLibrary.GetRunStateValue` (struct :`TagName` "Stat.Ability.Arrow.MaxDistance")) (`self.BaseBulletRange`))))