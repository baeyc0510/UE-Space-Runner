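; GA_GenerateMissile is a Gameplay Ability that recharges the player character's missiles through its missile manager.
; On activation it ends immediately if the manager is full; otherwise it starts a recharge and rebinds to the fired-missiles event, unbinding first to avoid duplicate bindings.
; Commit is deferred until that event fires, so cost and cooldown apply on firing, after which the ability ends.
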(event `self.K2_ActivateAbility`
  (bind _missilemanager (`self.MissileManager`))
  (`parent.K2_ActivateAbility`)
  (bind _asbp_player_character (cast `/Game/BP/Characters/Player/BP_PlayerCharacter` (`self.GetAvatarActorFromActorInfo`)))
  (bind _output_get (set `self.MissileManager` (`/Game/BP/Characters/Player/BP_PlayerCharacter.BP_MissileManager` _asbp_player_character)))
  (if (not (`/Game/BP/Combat/BP_MissileManager.IsFull` _output_get))
    (`/Game/BP/Combat/BP_MissileManager.RechargeMissiles` (`self.MissileManager`))
    (remove `/Game/BP/Combat/BP_MissileManager.OnFiredMissiles` _missilemanager (delegate `OnFiredMissiles`))
    (add `/Game/BP/Combat/BP_MissileManager.OnFiredMissiles` _missilemanager (delegate `OnFiredMissiles`))
    (else
      (`self.K2_EndAbility`))))

(event `OnFiredMissiles`
  (`self.K2_CommitAbility`)
  (`self.K2_EndAbility`))