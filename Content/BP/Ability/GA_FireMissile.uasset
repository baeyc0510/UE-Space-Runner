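; Gameplay ability that fires missiles from the player at an enemy in front, then ends immediately.
; A sphere overlap, sized by the detection-range stat, finds EnemyBase pawns and keeps those in the forward hemisphere.
; MinDistance drops to zero on the first match, so the first qualifying enemy wins rather than the nearest.
; BPMissileManager on BP_PlayerCharacter launches the missiles using Sword run-state stats for power, speed and range.
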(event `self.K2_ActivateAbility`
  (`|ExecutionSequence`
    (:`then_0`
      (set `self.TargetActor` null)
      (set `self.MinDistance` 1e+16)
      (bind _outactors (`KismetSystemLibrary.SphereOverlapActors` (`Actor.K2_GetActorLocation` (`self.GetAvatarActorFromActorInfo`)) (`self.GetMissileMaxDistance`) (`|MakeArray` "ObjectTypeQuery3" :!type "EObjectTypeQuery Enum") "/Script/Runner.EnemyBase"))
      (for _array_element _outactors
        (if (and (`self.IsInFrontOfAvatar` _array_element) (`self.IsInRange` _array_element))
          (set `self.TargetActor` _array_element)
          (set `self.MinDistance` 0.0))))
    (:`then_1`
      (`/Engine/EditorBlueprintResources/StandardMacros.IsValid` (`self.TargetActor`)
        (:`Is Valid`
          (bind _asbp_player_character (cast `/Game/BP/Characters/Player/BP_PlayerCharacter` (`self.GetAvatarActorFromActorInfo`)))
          (`/Game/BP/Combat/BP_MissileManager.FireMissiles` (`/Game/BP/Characters/Player/BP_PlayerCharacter.BP_MissileManager` _asbp_player_character) (`RogueliteBlueprintLibrary.GetRunStateValue` (struct :`TagName` "Stat.Ability.Sword.Power")) (`self.GetMissileSpeed`) (`self.GetMissileMaxDistance`) (`self.TargetActor`)))))
    (:`then_2`
      (`self.K2_EndAbility`))))

(fn `GetMissileMaxDistance`
  (returns (ReturnValue :type "Float (double-precision)"))
  (return (* (`RogueliteBlueprintLibrary.GetRunStateValue` (struct :`TagName` "Stat.Ability.Sword.DetectionRange") 1.0) (`self.BaseSwordRange`))))

(fn `GetMissileSpeed`
  (returns (ReturnValue :type "Float (double-precision)"))
  (return (* (`RogueliteBlueprintLibrary.GetRunStateValue` (struct :`TagName` "Stat.Ability.Sword.Speed")) (`self.BaseSwordSpeed`))))

(fn `IsInFrontOfAvatar`
  (params (InTargetActor :type "Actor Object Reference"))
  (returns (IsFront :type Boolean))
  (bind _returnvalue (`self.GetAvatarActorFromActorInfo`))
  (return (> (`KismetMathLibrary.Dot_VectorVector` (`KismetMathLibrary.Normal` (- (`Actor.K2_GetActorLocation` InTargetActor) (`Actor.K2_GetActorLocation` _returnvalue))) (`Actor.GetActorForwardVector` _returnvalue)) 0.0)))

(fn `IsInRange`
  (params (Target :type "Actor Object Reference"))
  (returns (IsInRange :type Boolean))
  (return (< (`KismetMathLibrary.Vector_Distance` (`Actor.K2_GetActorLocation` Target) (`Actor.K2_GetActorLocation` (`self.GetAvatarActorFromActorInfo`))) (`self.MinDistance`))))