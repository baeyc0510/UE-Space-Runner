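; Level tile that a TileGenerator chains via a next-tile point, with spawn transforms for boss, left and right spawns.
; Its box overlap notifies the generator when the player enters.
; Two child-actor reward doors are initialised with separate reward actions; touching either hitbox while enabled grants that door's reward and hides both, allowing one pick.
; The construction script scales the root and doors from the tile's size variables.
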(event `self.ReceiveBeginPlay`)

(event `self.Box.OnComponentBeginOverlap`
  (params (OverlappedComponent :type "PrimitiveComponent Object Reference") (OtherActor :type "Actor Object Reference") (OtherComp :type "PrimitiveComponent Object Reference") (OtherBodyIndex :type Integer) (bFromSweep :type Boolean) (SweepResult :type "HitResult Structure (by ref)"))
  (cast `/Game/BP/Characters/Player/BP_PlayerCharacter` OtherActor)
  (bind _tilegenerator (`self.TileGenerator`)
    (:`then`
      (`/Game/BP/Tiles/BP_TileGenerator.OnPlayerOverlapTile` _tilegenerator self))
    (:`else`)))

(event `self.DoorHitBox_R.OnComponentBeginOverlap`
  (params (OverlappedComponent :type "PrimitiveComponent Object Reference") (OtherActor :type "Actor Object Reference") (OtherComp :type "PrimitiveComponent Object Reference") (OtherBodyIndex :type Integer) (bFromSweep :type Boolean) (SweepResult :type "HitResult Structure (by ref)"))
  (bind _asbp_player_character (cast `/Game/BP/Characters/Player/BP_PlayerCharacter` OtherActor))
  (if (`self.bDoorEnabled`)
    (bind _asbp_reward_door (cast `/Game/BP/RewardActors/BP_RewardDoor` (`ChildActorComponent.ChildActor` (`self.DoorActor_R`))))
    (`/Game/BP/Characters/Player/BP_PlayerCharacter.GiveReward` _asbp_player_character (`/Game/BP/RewardActors/BP_RewardDoor.RewardAction` _asbp_reward_door))
    (`self.SetEnableDoors` false)))

(event `self.DoorHitBox_L.OnComponentBeginOverlap`
  (params (OverlappedComponent :type "PrimitiveComponent Object Reference") (OtherActor :type "Actor Object Reference") (OtherComp :type "PrimitiveComponent Object Reference") (OtherBodyIndex :type Integer) (bFromSweep :type Boolean) (SweepResult :type "HitResult Structure (by ref)"))
  (bind _asbp_player_character (cast `/Game/BP/Characters/Player/BP_PlayerCharacter` OtherActor))
  (if (`self.bDoorEnabled`)
    (bind _asbp_reward_door (cast `/Game/BP/RewardActors/BP_RewardDoor` (`ChildActorComponent.ChildActor` (`self.DoorActor_L`))))
    (`/Game/BP/Characters/Player/BP_PlayerCharacter.GiveReward` _asbp_player_character (`/Game/BP/RewardActors/BP_RewardDoor.RewardAction` _asbp_reward_door))
    (`self.SetEnableDoors` false)))

(fn `Get Left Spawn Transform`
  (returns (ReturnValue :type "Transform Structure"))
  (return (`KismetMathLibrary.MakeTransform` (.location (`SceneComponent.K2_GetComponentToWorld` (`self.SpawnPoint_Left`))) (.rotation (`SceneComponent.K2_GetComponentToWorld` (`self.SpawnPoint_Left`))))))

(fn `GetBossSpawnTransform`
  (returns (ReturnValue :type "Transform Structure"))
  (return (`KismetMathLibrary.MakeTransform` (.location (`SceneComponent.K2_GetComponentToWorld` (`self.SpawnPoint_Boss`))) (.rotation (`SceneComponent.K2_GetComponentToWorld` (`self.SpawnPoint_Boss`))))))

(fn `GetNextTileLocation`
  (returns (ReturnValue :type "Vector Structure"))
  (return (`SceneComponent.K2_GetComponentLocation` (`self.NextSpawnPoint`))))

(fn `GetRightSpawnTransform`
  (returns (ReturnValue :type "Transform Structure"))
  (return (`KismetMathLibrary.MakeTransform` (.location (`SceneComponent.K2_GetComponentToWorld` (`self.SpawnPoint_Right`))) (.rotation (`SceneComponent.K2_GetComponentToWorld` (`self.SpawnPoint_Right`))))))

(fn `InitDoors`
  (params (RewardAction1 :type "RogueliteActionData Object Reference") (RewardAction2 :type "RogueliteActionData Object Reference"))
  (`|ExecutionSequence`
    (:`then_0`
      (bind _asbp_reward_door (cast `/Game/BP/RewardActors/BP_RewardDoor` (`ChildActorComponent.ChildActor` (`self.DoorActor_L`))))
      (`/Game/BP/RewardActors/BP_RewardDoor.InitDoor` _asbp_reward_door RewardAction1))
    (:`then_1`
      (bind _asbp_reward_door_2 (cast `/Game/BP/RewardActors/BP_RewardDoor` (`ChildActorComponent.ChildActor` (`self.DoorActor_R`))))
      (`/Game/BP/RewardActors/BP_RewardDoor.InitDoor` _asbp_reward_door_2 RewardAction2))))

(fn `SetEnableDoors`
  (params (bEnable :type Boolean))
  (set `self.bDoorEnabled` bEnable)
  (`SceneComponent.SetVisibility` (`self.DoorActor_R`) (`self.bDoorEnabled`) true)
  (`SceneComponent.SetVisibility` (`self.DoorActor_L`) (`self.bDoorEnabled`) true))

(fn `UserConstructionScript`
  (bind _returnvalue (* (`self.TileWidthScale`) 0.9))
  (`SceneComponent.SetRelativeScale3D` (`self.DefaultSceneRoot`) (`KismetMathLibrary.MakeVector` (`self.TileHeightScale`) (`self.TileWidthScale`) 1.0))
  (`SceneComponent.SetWorldScale3D` (`self.DoorActor_R`) (`KismetMathLibrary.MakeVector` _returnvalue 1.0 1.0))
  (`SceneComponent.SetWorldScale3D` (`self.DoorActor_L`) (`KismetMathLibrary.MakeVector` _returnvalue 1.0 1.0)))