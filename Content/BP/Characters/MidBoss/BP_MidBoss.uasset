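; BP_MidBoss is a mid-boss character that offers the player a roguelite selection when it dies.
; On death it queries the Roguelite subsystem with the Pool.Boss tag, passes the result to OpenSelection on BP_PlayerCharacter, then destroys itself.
; The destroy runs only if the cast of player 0's character succeeds.
; BeginPlay only calls the parent, and the construction script adds a debug "Hello" print after its parent call.
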(event `self.ReceiveBeginPlay`
  (`parent.ReceiveBeginPlay`))

(event `self.K2_OnDie`
  (bind _returnvalue (`RogueliteSubsystem.ExecuteQuery` (subsystem `RogueliteSubsystem`) (make `RogueliteQuery` null (struct :`GameplayTags` (struct :`(TagName` "Pool.Boss"))))))
  (bind _asbp_player_character (cast `/Game/BP/Characters/Player/BP_PlayerCharacter` (`GameplayStatics.GetPlayerCharacter` 0)))
  (`/Game/BP/Characters/Player/BP_PlayerCharacter.OpenSelection` _asbp_player_character _returnvalue)
  (`self.K2_DestroyActor`))

(fn `UserConstructionScript`
  (`parent.UserConstructionScript`)
  (`KismetSystemLibrary.PrintString` "Hello"))