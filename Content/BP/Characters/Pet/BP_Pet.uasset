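; Companion pet character, a sci-fi dog that follows its owner and attacks enemies under an AI controller and blackboard.
; Walk speed tracks chase, catch-up or owner pace, and the pet teleports to its follow point when far behind and out of the owner's view.
; Attacks play a montage and send damage through CombatInterface, with power from a roguelite stat scaled by a level curve table.
; Level also selects the skin mesh.
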(event `self.ReceiveBeginPlay`)

(event `self.ReceivePossessed`
  (params (NewController :type "Controller Object Reference"))
  (bind _asbp_pet_aicontroller (cast `/Game/BP/Characters/Pet/AI/BP_PetAIController` NewController))
  (set `self.PetAIController` _asbp_pet_aicontroller))

(event `self.ReceiveTick`
  (params (DeltaSeconds :type "Float (single-precision)"))
  (`self.UpdateWalkSpeed`)
  ;[1 1 1] Teleport To owner
  (`/Engine/EditorBlueprintResources/StandardMacros.IsValid` (`self.OwnerCharacter`)
    (:`Is Valid`
      (if (and (not (`self.IsTargetInFrontOfSource` self (`self.OwnerCharacter`))) (> (`KismetMathLibrary.Vector_Distance2D` (`self.K2_GetActorLocation` (`self.OwnerCharacter`)) (`self.K2_GetActorLocation`)) 1200.0))
        (`self.K2_SetActorLocation` (`self.OwnerFollowLocation`))))))

(event `StartAttack`
  (params (TargetActor :type "Actor Object Reference"))
  (bind _output_get (set `self.AttackTarget` TargetActor))
  (`/Engine/EditorBlueprintResources/StandardMacros.IsValid` _output_get
    (:`Is Valid`
      (`|PlayMontage` (`self.Mesh`) "/Game/BP/Characters/Pet/Animations/Montages/AM_PetAttack.AM_PetAttack"
        (:`OnCompleted`
          _)
        (:`OnInterrupted`
          _))
      (set `self.AttackTarget` null)
      (`self.OnAttackFinished`))
    (:`Is Not Valid`
      (`self.OnAttackFinished`))))

(event `OnAttack`
  (bind _attacktarget (`self.AttackTarget`)
    (:`then`
      (if (`KismetSystemLibrary.DoesImplementInterface` _attacktarget "/Script/Runner.CombatInterface")
        (bind _output_get (set `self.DamageContext` (`CombatBlueprintLibrary.CreateDamageContext` self (`self.AttackTarget`) null)))
        (`CombatBlueprintLibrary.SetDamageContextSourceValue` _output_get (`BlueprintGameplayTagLibrary.MakeLiteralGameplayTag` (struct :`TagName` "Data.BaseDamage")) (`self.GetAttackPower`))
        (message `CombatInterface.ApplyDamage` (`self.AttackTarget`) (`self.DamageContext`))))
    (:`else`
      (`self.OnAttackFinished`))))

(fn `GetAttackPower`
  (returns (ReturnValue :type "Float (double-precision)"))
  (bind _returnvalue (`RogueliteStatReceiverComponent.GetStat` (`self.RogueliteStatReceiver`) (struct :`TagName` "Pet.Stat.Attack.Power") 1.0))
  (bind _outxy (`DataTableFunctionLibrary.EvaluateCurveTableRow` "/Game/Data/LevelData/CT_PetLevelTable.CT_PetLevelTable" "AttackPowerMultiplier" (`KismetMathLibrary.Conv_IntToDouble` (`self.Level`)))
    (:`RowFound`
      (return (* _outxy _returnvalue)))
    (:`RowNotFound`
      (return _returnvalue))))

(fn `GetIndex`
  (returns (PetIndex :type Integer))
  (return (`self.PetIndex`)))

(fn `GetOwnerFollowLocation`
  (returns (OwnerFollowLocation :type "Vector Structure"))
  (`/Engine/EditorBlueprintResources/StandardMacros.IsValid` (`self.OwnerCharacter`)
    (:`Is Valid`
      (return (`self.OwnerFollowLocation`)))
    (:`Is Not Valid`
      (return (`self.K2_GetActorLocation`)))))

(fn `HasTarget`
  (returns (ReturnValue :type Boolean))
  (`self.TargetEnemyToChase`
    (:`then`
      (return true))
    (:`else`
      (return false))))

(fn `InitPet`
  (params (OwnerCharacter :type "Character Object Reference") (Level :type Integer))
  (bind _returnvalue (`AIBlueprintHelperLibrary.GetBlackboard` null))
  (`|ExecutionSequence`
    (:`then_0`
      (bind _output_get (set `self.OwnerCharacter` OwnerCharacter))
      (`/Engine/EditorBlueprintResources/StandardMacros.IsValid` _returnvalue
        (:`Is Valid`
          (`BlackboardComponent.SetValueAsObject` _returnvalue "OwnerActor" _output_get))))
    (:`then_1`
      (`self.SetLevel` Level))))

(fn `IsTargetInFrontOfSource`
  (params (TargetActor :type "Actor Object Reference") (SourceActor :type "Actor Object Reference"))
  (returns (ReturnValue :type Boolean))
  (return (> (`KismetMathLibrary.Dot_VectorVector` (`KismetMathLibrary.Normal` (- (`self.K2_GetActorLocation` TargetActor) (`self.K2_GetActorLocation` SourceActor))) (`self.GetActorForwardVector` SourceActor)) 0.0)))

(fn `SetBlackBoardIsAttackPlaying`
  (params (BoolValue :type Boolean))
  (bind _returnvalue (`self.GetController`))
  (bind _returnvalue_2 (`AIBlueprintHelperLibrary.GetBlackboard` _returnvalue))
  (`/Engine/EditorBlueprintResources/StandardMacros.IsValid` _returnvalue
    (:`Is Valid`
      (`/Engine/EditorBlueprintResources/StandardMacros.IsValid` _returnvalue_2
        (:`Is Valid`
          (`BlackboardComponent.SetValueAsBool` _returnvalue_2 "IsAttackPlaying" BoolValue))))))

(fn `SetIndex`
  (params (PetIndex :type Integer))
  (set `self.PetIndex` PetIndex))

(fn `SetLevel`
  (params (Level :type Integer))
  (bind _mesh (`self.Mesh`))
  (set `self.Level` Level)
  (switch `int` (`self.Level`)
    (:`Default`
      (`SkeletalMeshComponent.SetSkeletalMeshAsset` _mesh "/Game/SciFi_Dog/Mesh/SK_SciFi_Dog_Skin1.SK_SciFi_Dog_Skin1" :!label _label))
    (:`1`
      (goto _label))
    (:`2`
      (`SkeletalMeshComponent.SetSkeletalMeshAsset` _mesh "/Game/SciFi_Dog/Mesh/SK_SciFi_Dog_Skin4.SK_SciFi_Dog_Skin4"))
    (:`3`
      (`SkeletalMeshComponent.SetSkeletalMeshAsset` _mesh "/Game/SciFi_Dog/Mesh/SK_SciFi_Dog_Skin3.SK_SciFi_Dog_Skin3"))))

(fn `SetOwnerFollowLocation`
  (params (OwnerFollowLocation :type "Vector Structure"))
  (set `self.OwnerFollowLocation` OwnerFollowLocation))

(fn `UpdateWalkSpeed`
  (locals (OwnerSpeed :type "Float (single-precision)" :default 0.0) (DistanceToOwner :type "Float (double-precision)" :default 0.0))
  (if (`self.HasTarget`)
    (set `CharacterMovementComponent.MaxWalkSpeed` (`self.ChaseSpeed`) (`self.CharacterMovement`))
    (else
      (bind _ownercharacter (`self.OwnerCharacter`)
        (:`then`
          (set `local.OwnerSpeed` (`CharacterMovementComponent.MaxWalkSpeed` (`Character.CharacterMovement` _ownercharacter)))
          (bind _output_get (set `local.DistanceToOwner` (`KismetMathLibrary.Vector_Distance2D` (`self.K2_GetActorLocation` (`self.OwnerCharacter`)) (`self.K2_GetActorLocation`))))
          (if (> _output_get (`self.AcceptableDistanceToOwner`))
            (set `CharacterMovementComponent.MaxWalkSpeed` (+ (`local.OwnerSpeed`) (`self.FollowUpSpeed`)) (`self.CharacterMovement`))
            (else
              (set `CharacterMovementComponent.MaxWalkSpeed` (`local.OwnerSpeed`) (`self.CharacterMovement`)))))
        (:`else`)))))

(fn `UserConstructionScript`)