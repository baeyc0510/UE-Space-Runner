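; AI controller for pet characters that runs the pet behavior tree and keeps its blackboard in sync with the pet.
; On possess it caches the BP_Pet, and on BeginPlay it starts BT_Pet.
; Each tick it copies the pet's owner follow location and enemy chase target into the blackboard, clearing the target when invalid.
; It also exposes a separate TargetActor setter and getter, which the blackboard update does not use.
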(event `self.ReceivePossess`
  (params (PossessedPawn :type "Pawn Object Reference"))
  (bind _asbp_pet (cast `/Game/BP/Characters/Pet/BP_Pet` PossessedPawn))
  (set `self.OwnerPet` _asbp_pet))

(event `self.ReceiveBeginPlay`
  (`self.RunBehaviorTree` "/Game/BP/Characters/Pet/AI/BT_Pet.BT_Pet"))

(event `self.ReceiveTick`
  (params (DeltaSeconds :type "Float (single-precision)"))
  (`self.SetBBOwnerFollowLocation`)
  (`self.SetBBTargetActor`))

(fn `GetTargetActor`
  (returns (TargetActor :type "Actor Object Reference") (IsValidActor :type Boolean))
  (bind _targetactor (`self.TargetActor`))
  (return _targetactor (`KismetSystemLibrary.IsValid` _targetactor)))

(fn `SetBBOwnerFollowLocation`
  (bind _returnvalue (`AIBlueprintHelperLibrary.GetBlackboard` null))
  (`/Engine/EditorBlueprintResources/StandardMacros.IsValid` (`self.OwnerPet`)
    (:`Is Valid`
      (`/Engine/EditorBlueprintResources/StandardMacros.IsValid` _returnvalue
        (:`Is Valid`
          (`BlackboardComponent.SetValueAsVector` _returnvalue "OwnerFollowLocation" (`/Game/BP/Characters/Pet/BP_Pet.GetOwnerFollowLocation` (`self.OwnerPet`))))))))

(fn `SetBBTargetActor`
  (bind _returnvalue (`AIBlueprintHelperLibrary.GetBlackboard` null))
  (bind _targetenemytochase (`/Game/BP/Characters/Pet/BP_Pet.TargetEnemyToChase` (`self.OwnerPet`)))
  (`/Engine/EditorBlueprintResources/StandardMacros.IsValid` (`self.OwnerPet`)
    (:`Is Valid`
      (`/Engine/EditorBlueprintResources/StandardMacros.IsValid` _returnvalue
        (:`Is Valid`
          (`/Engine/EditorBlueprintResources/StandardMacros.IsValid` _targetenemytochase
            (:`Is Valid`
              (`BlackboardComponent.SetValueAsObject` _returnvalue "TargetActor" _targetenemytochase))
            (:`Is Not Valid`
              (`BlackboardComponent.SetValueAsObject` _returnvalue "TargetActor" null))))))))

(fn `SetTargetActor`
  (params (TargetActor :type "Actor Object Reference"))
  (set `self.TargetActor` TargetActor))

(fn `UserConstructionScript`)