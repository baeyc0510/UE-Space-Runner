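; Player character for a runner game that moves forward constantly with lateral input, while the camera boom's Y stays fixed.
; Each tick it updates movement, retries passive GAS abilities granted at BeginPlay and reports distance progress to BP_RunnerGameState.
; A health text widget follows HealthComponent changes, and action rewards are acquired directly or through a selection widget that pauses the game.
; On death, score converts to currency and a game-over screen appears.
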(event `self.ReceiveBeginPlay`
  (`self.InitHealthWidget`)
  (set `self.StartPosX` (.x (`self.K2_GetActorLocation`)))
  (set `self.CameraY` (.y (`self.K2_GetActorLocation`)))
  (`self.GiveAbilities`)
  (bind _asbp_runner_game_state (cast `/Game/BP/GameFramework/Gameplay/BP_RunnerGameState` (`GameplayStatics.GetGameState`)))
  (set `self.RunnerGameState` _asbp_runner_game_state))

(event `self.ReceiveTick`
  (params (DeltaSeconds :type "Float (single-precision)"))
  (`self.UpdateLocation`)
  (`self.ActivatePassiveAbilities`)
  (`self.UpdateProgress`))

(event `PauseAndSetUIMode`
  (bind _returnvalue (`GameplayStatics.GetPlayerController` 0))
  (`GameplayStatics.SetGamePaused` true)
  (set `PlayerController.bShowMouseCursor` true _returnvalue)
  (`WidgetBlueprintLibrary.SetInputMode_UIOnlyEx` _returnvalue (`self.SelectionWidget`)))

(event `self.K2_OnDie`
  (bind _asbp_runner_game_state (cast `/Game/BP/GameFramework/Gameplay/BP_RunnerGameState` (`GameplayStatics.GetGameState`)))
  (bind _output_get (set `self.CurrencyToAdd` (/ (`/Game/BP/GameFramework/Gameplay/BP_RunnerGameState.CurrentScore` _asbp_runner_game_state) 100)))
  (`RogueliteBlueprintLibrary.AddRunStateValue` (struct :`TagName` "GameState.Currency") (`KismetMathLibrary.Conv_IntToDouble` _output_get))
  (bind _returnvalue (`|CreateWidget` "/Game/BP/UI/GameOver/W_GameOver.W_GameOver_C" null (`KismetTextLibrary.Conv_IntToText` (`self.CurrencyToAdd`))))
  (`UserWidget.AddToViewport` _returnvalue 0))

(fn `ActivatePassiveAbilities`
  (for _array_element (`self.PassiveAbilitySpecs`)
    (`AbilitySystemComponent.TryActivateAbility` (`self.AbilitySystemComponent`) _array_element true)))

(fn `GetFirePoint`
  (returns (ReturnValue :type "Vector Structure"))
  (return (`SceneComponent.K2_GetComponentLocation` (`self.FirePoint`))))

(fn `GiveAbilities`
  (for _array_element (`self.StartupPassiveAbilities`)
    (bind _returnvalue (`AbilitySystemComponent.K2_GiveAbility` (`self.AbilitySystemComponent`) _array_element 0 -1))
    (`KismetArrayLibrary.Array_Add` (`self.PassiveAbilitySpecs`) _returnvalue)))

(fn `GiveReward`
  (params (RewardAction :type "RogueliteActionData Object Reference"))
  (`RogueliteBlueprintLibrary.AcquireAction` RewardAction))

(fn `InitHealthWidget`
  (bind _asw_text (cast `/Game/BP/UI/W_Text` (`WidgetComponent.GetWidget` (`self.HealthWidgetComponent`))))
  (bind _output_get (set `self.HealthWidget` _asw_text))
  (`/Game/BP/UI/W_Text.SetContent` _output_get (`KismetTextLibrary.Conv_Int64ToText` (`KismetMathLibrary.Round64` (`HealthComponent.GetCurrentHealth` (`self.HealthComponent`)))) (`self.HealthColor`))
  (add `HealthComponent.OnHealthChanged` (`self.HealthComponent`) (`|CreateDelegate` :!event `OnHealthChanged`)))

(fn `OnHealthChanged`
  (params (CurrentHealth :type "Float (single-precision)") (MaxHealth :type "Float (single-precision)") (DeltaHealth :type "Float (single-precision)"))
  (bind _healthwidget (`self.HealthWidget`)
    (:`then`
      (`/Game/BP/UI/W_Text.SetContent` _healthwidget (`KismetTextLibrary.Conv_Int64ToText` (`KismetMathLibrary.Round64` CurrentHealth)) (`self.HealthColor`)))
    (:`else`)))

(fn `OnSelectAction`
  (params (SelectedAction :type "/Game/Data/RogueliteActions/BP_RunnerActionData Object Reference"))
  (bind _returnvalue (`GameplayStatics.GetPlayerController` 0))
  (`RogueliteBlueprintLibrary.AcquireAction` SelectedAction)
  (bind _selectionwidget (`self.SelectionWidget`)
    (:`then`
      (`Widget.RemoveFromParent` _selectionwidget)
      (`GameplayStatics.SetGamePaused` false)
      (set `PlayerController.bShowMouseCursor` false _returnvalue)
      (`WidgetBlueprintLibrary.SetInputMode_GameOnly` _returnvalue))
    (:`else`)))

(fn `OpenSelection`
  (params (Choices :type "Array of RogueliteActionData Object Reference (by ref)"))
  (if (`KismetArrayLibrary.Array_IsNotEmpty` Choices)
    (bind _returnvalue (`|CreateWidget` "/Game/BP/UI/Selection/W_SelectAction.W_SelectAction_C"))
    (bind _output_get (set `self.SelectionWidget` _returnvalue))
    (`/Game/BP/UI/Selection/W_SelectAction.SetSelections` _output_get Choices)
    (add `/Game/BP/UI/Selection/W_SelectAction.OnSelectAction` _output_get (`|CreateDelegate` :!event `OnSelectAction`))
    (`UserWidget.AddToViewport` (`self.SelectionWidget`) 0)
    (`KismetSystemLibrary.K2_SetTimerForNextTickDelegate` (`|CreateDelegate` :!event `PauseAndSetUIMode`))))

(fn `UpdateLocation`
  (bind _cameraboom (`self.CameraBoom`))
  (bind _movementvector_x (`KismetMathLibrary.BreakVector2D` (`self.MovementVector`)))
  (set `MovementComponent.Velocity` (+ (* (`self.GetActorRightVector`) (* (`CharacterMovementComponent.MaxWalkSpeed` (`self.CharacterMovement`)) _movementvector_x)) (* (`self.GetActorForwardVector`) (`CharacterMovementComponent.MaxWalkSpeed` (`self.CharacterMovement`)))) (`self.CharacterMovement`))
  (`SceneComponent.K2_SetWorldLocation` _cameraboom (`KismetMathLibrary.MakeVector` (.x (`SceneComponent.K2_GetComponentLocation` _cameraboom)) (`self.CameraY`) (.z (`SceneComponent.K2_GetComponentLocation` _cameraboom))) false false))

(fn `UpdateProgress`
  (bind _runnergamestate (`self.RunnerGameState`)
    (:`then`
      (`/Game/BP/GameFramework/Gameplay/BP_RunnerGameState.UpdateProgress` _runnergamestate (`self.StartPosX`) (.x (`self.K2_GetActorLocation`))))
    (:`else`)))

(fn `UserConstructionScript`)