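; BP_EnemyCharacter is an enemy character that awards score and can leave a reward box when killed.
; The HealthComponent's death delegate adds the enemy's truncated max health to the BP_RunnerGameState score.
; A separate OnDie event runs a roguelite query on the Pool.Chest tag, spawning BP_RewardBox with the first result as its reward action.
; OnDie then removes the enemy via a near-zero lifespan.
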(event `self.ReceiveBeginPlay`
  (`parent.ReceiveBeginPlay`)
  (add `HealthComponent.OnDeath` (`self.HealthComponent`) (delegate `OnDeath_Event`)))

(event `OnDeath_Event`
  (bind _asbp_runner_game_state (cast `/Game/BP/GameFramework/Gameplay/BP_RunnerGameState` (`GameplayStatics.GetGameState`)))
  (`/Game/BP/GameFramework/Gameplay/BP_RunnerGameState.AddScore` _asbp_runner_game_state (`KismetMathLibrary.FTrunc` (`HealthComponent.GetMaxHealth` (`self.HealthComponent`)))))

(event `self.K2_OnDie`
  (`|ExecutionSequence`
    (:`then_0`
      (bind _returnvalue (`RogueliteBlueprintLibrary.ExecuteQuery` (make `RogueliteQuery` null (struct :`GameplayTags` (struct :`(TagName` "Pool.Chest"))) 1)))
      (if (`KismetArrayLibrary.Array_IsNotEmpty` _returnvalue)
        (`|SpawnActorFromClass` "/Game/BP/RewardActors/BP_RewardBox.BP_RewardBox_C" (`KismetMathLibrary.MakeTransform` (`self.K2_GetActorLocation`) (`self.K2_GetActorRotation`)) "Undefined" "MultiplyWithRoot" null (`|GetArrayItem` _returnvalue) null)))
    (:`then_1`
      (`self.SetLifeSpan` 0.01))))

(fn `UserConstructionScript`
  (`parent.UserConstructionScript`))