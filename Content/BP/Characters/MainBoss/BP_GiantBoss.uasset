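; BP_GiantBoss is a boss character that offers the player a roguelite selection when it dies.
; Its OnDie event queries the roguelite subsystem for the Pool.Boss tag and passes the result to OpenSelection on player 0's BP_PlayerCharacter, then destroys the boss.
; If that player cast fails, the boss is not destroyed here.
; The graph holds no other active logic beyond the parent construction script call.
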(event `self.K2_OnDie`
  (bind _returnvalue (`RogueliteSubsystem.ExecuteQuery` (subsystem `RogueliteSubsystem`) (make `RogueliteQuery` null (struct :`GameplayTags` (struct :`(TagName` "Pool.Boss"))))))
  (bind _asbp_player_character (cast `/Game/BP/Characters/Player/BP_PlayerCharacter` (`GameplayStatics.GetPlayerCharacter` 0)))
  (`/Game/BP/Characters/Player/BP_PlayerCharacter.OpenSelection` _asbp_player_character _returnvalue)
  (`self.K2_DestroyActor`))

(fn `UserConstructionScript`
  (`parent.UserConstructionScript`))