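; BP_EnemyBase is a base enemy whose remaining health doubles as the damage it deals to the player.
; InitEnemyByLevel sets max health from a wave scaling formula combining linear and exponential growth by level.
; A text widget shows rounded current health, updated through the HealthComponent's change event.
; When the HitBox overlaps the player, it sends current health as base damage through a damage context, then destroys itself.
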(event `self.ReceiveBeginPlay`
  (`parent.ReceiveBeginPlay`)
  (`self.SpawnDefaultController`)
  (bind _asw_text (cast `/Game/BP/UI/W_Text` (`WidgetComponent.GetWidget` (`self.HealthWidgetComponent`))))
  (bind _output_get (set `self.HealthWidget` _asw_text))
  (`/Game/BP/UI/W_Text.SetContent` _output_get (`KismetTextLibrary.Conv_Int64ToText` (`KismetMathLibrary.Round64` (`HealthComponent.GetCurrentHealth` (`self.HealthComponent`)))) (struct :`R` 1.0 :`G` 1.0 :`B` 1.0 :`A` 1.0))
  (add `HealthComponent.OnHealthChanged` (`self.HealthComponent`) (delegate `OnHealthChanged_Event`)))

(event `OnHealthChanged_Event`
  (params (CurrentHealth :type "Float (single-precision)") (MaxHealth :type "Float (single-precision)") (DeltaHealth :type "Float (single-precision)"))
  (bind _healthwidget (`self.HealthWidget`)
    (:`then`
      (`/Game/BP/UI/W_Text.SetContent` _healthwidget (`KismetTextLibrary.Conv_Int64ToText` (`KismetMathLibrary.Round64` CurrentHealth)) (struct :`R` 1.0 :`G` 1.0 :`B` 1.0 :`A` 1.0)))
    (:`else`)))

(event `self.HitBox.OnComponentBeginOverlap`
  (params (OverlappedComponent :type "PrimitiveComponent Object Reference") (OtherActor :type "Actor Object Reference") (OtherComp :type "PrimitiveComponent Object Reference") (OtherBodyIndex :type Integer) (bFromSweep :type Boolean) (SweepResult :type "HitResult Structure (by ref)"))
  (bind _asbp_player_character (cast `/Game/BP/Characters/Player/BP_PlayerCharacter` OtherActor))
  (bind _output_get (set `self.DamageContext` (`CombatBlueprintLibrary.CreateDamageContext` self _asbp_player_character null)))
  (`BlueprintMapLibrary.Map_Add` (`.SourceValues` (break `DamageContext` _output_get)) (struct :`TagName` "Data.BaseDamage") (`HealthComponent.GetCurrentHealth` (`self.HealthComponent`)))
  (`CombatInterface.ApplyDamage` _asbp_player_character (`self.DamageContext`))
  (`self.K2_DestroyActor`))

(fn `CalcHealth`
  (params (InLevel :type Integer))
  (returns (Health :type "Float (double-precision)"))
  ;[0.08618 0.2865 1] Health = BaseHealth * (1 + (Level * LinearFactor)) * Pow(ExpFactor, Level / DivisionFactor)
  (return (* (* (`self.BaseHealth`) (+ 1.0 (* (`KismetMathLibrary.Conv_IntToDouble` InLevel) (`self.WaveLinearFactor`)))) (`KismetMathLibrary.MultiplyMultiply_FloatFloat` (`self.WaveExpFactor`) (`KismetMathLibrary.SafeDivide` (`KismetMathLibrary.Conv_IntToDouble` InLevel) (`KismetMathLibrary.Conv_IntToDouble` (`self.WaveDivisionFactor`)))))))

(fn `InitEnemyByLevel`
  (params (Level :type Integer))
  (bind _output_get (set `self.Level` Level))
  (`HealthComponent.SetMaxHealth` (`self.HealthComponent`) (`self.CalcHealth` _output_get) true))

(fn `UserConstructionScript`)