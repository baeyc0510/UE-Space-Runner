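; BP_EnemySpawnManager spawns leveled enemies and tracks them by spawn key so each group can be destroyed together.
; SpawnEnemy creates the actor, initializes BP_EnemyBase instances by level and stores them in a map of STSpawnPool structs, destroying actors of other classes.
; DestorySpawnedActorsByKey destroys a key's valid actors in reverse order, then removes the map entry.
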(fn `DestorySpawnedActorsByKey`
  (params (SpawnKey :type Name))
  (bind (_value _returnvalue) (`BlueprintMapLibrary.Map_Find` (`self.SpawnedActors`) SpawnKey))
  (if _returnvalue
    (bind (_arrayindex _arrayelement) (`/Engine/EditorBlueprintResources/StandardMacros.ReverseForEachLoop` (`.Actors_3_0BBDFE554A53C177810A1BBE2835BBA3` (break `/Game/BP/Combat/ST_SpawnPool` _value)))
      (:`LoopBody`
        (`/Engine/EditorBlueprintResources/StandardMacros.IsValid` _arrayelement
          (:`Is Valid`
            (`Actor.K2_DestroyActor` _arrayelement))))
      (:`Completed`
        (`BlueprintMapLibrary.Map_Remove` (`self.SpawnedActors`) (`local.SpawnKey`))))))

(fn `SpawnEnemy`
  (params (SpawnKey :type Name) (EnemyClass :type "/Game/BP/Characters/BP_EnemyBase Class Reference") (SpawnTransform :type "Transform Structure") (EnemyLevel :type Integer))
  (locals (Pool :type "/Game/BP/Combat/ST_SpawnPool Structure") (SpawnedEnemy :type "/Game/BP/Characters/BP_EnemyBase Object Reference"))
  (bind (_value _returnvalue) (`BlueprintMapLibrary.Map_Find` (`self.SpawnedActors`) (`local.SpawnKey`)))
  (bind _returnvalue_2 (`|SpawnActorFromClass` EnemyClass SpawnTransform "AdjustIfPossibleButAlwaysSpawn" "MultiplyWithRoot" null null))
  (bind _asbp_enemy_base (cast `/Game/BP/Characters/BP_EnemyBase` _returnvalue_2)
    (:`then`
      (set `local.SpawnedEnemy` _asbp_enemy_base)
      (`|ExecutionSequence`
        (:`then_0`
          (`/Game/BP/Characters/BP_EnemyBase.InitEnemyByLevel` (`local.SpawnedEnemy`) (`local.EnemyLevel`))
          (if _returnvalue
            (bind _output_get (set `local.Pool` _value))
            (`KismetArrayLibrary.Array_Add` (`.Actors_3_0BBDFE554A53C177810A1BBE2835BBA3` (break `/Game/BP/Combat/ST_SpawnPool` _output_get)) (`local.SpawnedEnemy`))
            (else
              (set `local.Pool` (make `/Game/BP/Combat/ST_SpawnPool` (`|MakeArray` (`local.SpawnedEnemy`) :!type "Actor Object Reference"))))))
        (:`then_1`
          (`BlueprintMapLibrary.Map_Add` (`self.SpawnedActors`) (`local.SpawnKey`) (`local.Pool`)))))
    (:`CastFailed`
      (`Actor.K2_DestroyActor` _returnvalue_2))))