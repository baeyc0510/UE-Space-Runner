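; Pet manager component that spawns and destroys BP_Pet actors as roguelite pet actions are gained or lost, including those acquired before BeginPlay.
; A third stack of a pet action evolves into the next-level action, or tags Pet.FullyAcquired at max level and stacks.
; Each tick arranges pets in a semicircle behind the owner.
; Periodic forward sphere overlaps pick the nearest enemy as the shared chase target.
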(event `self.ReceiveBeginPlay`
  (add `RogueliteSubsystem.OnActionAcquired` (subsystem `RogueliteSubsystem`) (`|CreateDelegate` :!event `OnActionAcquired`))
  (add `RogueliteSubsystem.OnActionRemoved` (subsystem `RogueliteSubsystem`) (`|CreateDelegate` :!event `On Action Removed`))
  (`self.ProcessPreAcquiredActions`))

(event `self.ReceiveEndPlay`
  (params (EndPlayReason :type "EEndPlayReason Enum" :default "Destroyed"))
  (remove `RogueliteSubsystem.OnActionAcquired` (subsystem `RogueliteSubsystem`) (`|CreateDelegate` :!event `OnActionAcquired`))
  (remove `RogueliteSubsystem.OnActionRemoved` (subsystem `RogueliteSubsystem`) (`|CreateDelegate` :!event `On Action Removed`)))

(event `self.ReceiveTick`
  (params (DeltaSeconds :type "Float (single-precision)"))
  (`self.UpdateOwnerFollowLocations`)
  (`self.LostTarget`)
  (`|ExecutionSequence`
    (:`then_0`
      (bind _output_get (set `self.AccTime` (+ (`self.AccTime`) (`GameplayStatics.GetWorldDeltaSeconds`))))
      (if (>= _output_get (`self.SearchInterval`))
        (set `self.AccTime` 0.0)
        (`/Engine/EditorBlueprintResources/StandardMacros.IsValid` (`self.TargetActor`)
          (:`Is Not Valid`
            (`self.Search Target`)))))
    (:`then_1`
      (`self.SetTargetToPets`))))

(fn `FindNextLevelAction`
  (params (CurrentAction :type "RogueliteActionData Object Reference (by ref)"))
  (returns (FoundAction :type "RogueliteActionData Object Reference") (bFound :type Boolean))
  (locals (NextLevel :type Integer64))
  (set `local.NextLevel` (+ (`RogueliteActionData.GetValueAsInt` CurrentAction (struct :`TagName` "Pet.Stat.Level") 0) 1))
  (bind _result (`BlueprintSetLibrary.Set_ToArray` (`self.PetAcquireActions`)))
  (for _array_element _result
    (if (== (`RogueliteActionData.GetValueAsInt` _array_element (struct :`TagName` "Pet.Stat.Level") 0) (`local.NextLevel`))
      (return _array_element true)))
  (return null false))

(fn `GetSpawnedActionStack`
  (params (ActionToCheck :type "RogueliteActionData Object Reference"))
  (returns (Stack :type Integer))
  (locals (ActionToCheck :type "RogueliteActionData Object Reference") (ActionStack :type Integer))
  (for _array_element (`self.SpawnedPets`)
    (if (== (`.AcquireAction_2_4E3483554D0CFD4DD70897A143C601C1` (break `/Game/BP/Characters/Pet/ST_PetSpawnInfo` _array_element)) (`local.ActionToCheck`))
      (`/Engine/EditorBlueprintResources/StandardMacros.IncrementInt` (`local.ActionStack`))))
  (return (`local.ActionStack`)))

(fn `IsActorInBehindOfSource`
  (params (TargetActor :type "Actor Object Reference") (SourceActor :type "Actor Object Reference"))
  (returns (ReturnValue :type Boolean))
  (return (< (`KismetMathLibrary.Dot_VectorVector` (`KismetMathLibrary.Normal` (- (`Actor.K2_GetActorLocation` TargetActor) (`Actor.K2_GetActorLocation` SourceActor))) (`Actor.GetActorForwardVector` SourceActor)) 0.0)))

(fn `IsActorInFrontOfSource`
  (params (TargetActor :type "Actor Object Reference") (SourceActor :type "Actor Object Reference"))
  (returns (ReturnValue :type Boolean))
  (return (> (`KismetMathLibrary.Dot_VectorVector` (`KismetMathLibrary.Normal` (- (`Actor.K2_GetActorLocation` TargetActor) (`Actor.K2_GetActorLocation` SourceActor))) (`Actor.GetActorForwardVector` SourceActor)) 0.0)))

(fn `IsClosestTarget`
  (params (ActorToCheck :type "Actor Object Reference") (CurrentMinDistance :type "Float (double-precision)"))
  (returns (IsClosest :type Boolean) (NewMinDistance :type "Float (double-precision)"))
  (bind _returnvalue (`KismetMathLibrary.Vector_Distance2D` (`Actor.K2_GetActorLocation` (`self.GetOwner`)) (`Actor.K2_GetActorLocation` ActorToCheck)))
  (if (< _returnvalue (`local.CurrentMinDistance`))
    (return true _returnvalue)
    (else
      (return false (`local.CurrentMinDistance`)))))

(fn `LostTarget`
  (locals (OwnerActor :type "Actor Object Reference"))
  (set `local.OwnerActor` (`self.GetOwner`))
  (`/Engine/EditorBlueprintResources/StandardMacros.IsValid` (`self.TargetActor`)
    (:`Is Valid`
      (if (`self.IsActorInBehindOfSource` (`local.OwnerActor`) (`self.TargetActor`))
        (set `self.TargetActor` null)
        (`self.Search Target`)))
    (:`Is Not Valid`
      (set `self.TargetActor` null))))

(fn `NewFunction`)

(fn `On Action Removed`
  (params (Action :type "RogueliteActionData Object Reference") (OldStacks :type Integer) (NewStacks :type Integer))
  (locals (RemovedStack :type Integer) (RemovedAction :type "RogueliteActionData Object Reference") (SpawnInfoToRemove :type "/Game/BP/Characters/Pet/ST_PetSpawnInfo Structure") (ActorToDestroy :type "/Game/BP/Characters/Pet/BP_Pet Object Reference"))
  (bind _actortodestroy (`local.ActorToDestroy`))
  (set `local.RemovedAction` Action)
  (set `local.RemovedStack` (- OldStacks NewStacks))
  (if (`BlueprintSetLibrary.Set_Contains` (`self.PetAcquireActions`) Action)
    (for _ (range 1 (+ (`local.RemovedStack`) 1))
      (bind (_arrayindex _arrayelement) (`/Engine/EditorBlueprintResources/StandardMacros.ReverseForEachLoop` (`self.SpawnedPets`))
        (:`LoopBody`
          (if (== (`.AcquireAction_2_4E3483554D0CFD4DD70897A143C601C1` (break `/Game/BP/Characters/Pet/ST_PetSpawnInfo` _arrayelement)) (`local.RemovedAction`))
            (bind _output_get (set `local.SpawnInfoToRemove` _arrayelement))
            (set `local.ActorToDestroy` (`.SpawnedPet_5_8E52DBFB40CBD44121F6ABBD2ECF7630` (break `/Game/BP/Characters/Pet/ST_PetSpawnInfo` _output_get)))
            (bind _returnvalue (`KismetArrayLibrary.Array_RemoveItem` (`self.SpawnedPets`) (`local.SpawnInfoToRemove`)))
            (set `self.bRemovedPet` _returnvalue)
            (set `self.LastRemovedPetTransform` (`Actor.GetTransform` _actortodestroy))
            (`Actor.K2_DestroyActor` _actortodestroy)))))))

(fn `OnActionAcquired`
  (params (Action :type "RogueliteActionData Object Reference") (OldStacks :type Integer) (NewStacks :type Integer))
  (locals (AcquiredAction :type "RogueliteActionData Object Reference"))
  (bind _acquiredaction (`local.AcquiredAction`))
  (bind (_foundaction _bfound) (`self.FindNextLevelAction` (`local.AcquiredAction`)))
  (set `local.AcquiredAction` Action)
  (if (`BlueprintSetLibrary.Set_Contains` (`self.PetAcquireActions`) (`local.AcquiredAction`))
    (`|ExecutionSequence`
      (:`then_0`
        (if (== (`self.GetSpawnedActionStack` (`local.AcquiredAction`)) 2)
          ;[1 1 1] 진화
          (if _bfound
            (bind _returnvalue (`RogueliteBlueprintLibrary.AcquireAction` _foundaction))
            (if _returnvalue
              (`RogueliteBlueprintLibrary.RemoveAction` (`local.AcquiredAction`) 3 true)
              (return))
            (elif (== (`self.GetSpawnedActionStack` _acquiredaction) (`RogueliteActionData.MaxStacks` _acquiredaction))
              (if (not (`RogueliteBlueprintLibrary.HasTagInSystem` (struct :`TagName` "Pet.FullyAcquired")))
                (`RogueliteBlueprintLibrary.AddTagToSystem` (struct :`TagName` "Pet.FullyAcquired")))))))
      (:`then_1`
        (`self.SpawnPetFromAction` (`local.AcquiredAction`))))))

(fn `ProcessPreAcquiredActions`
  (locals (ActionToAcquire :type "RogueliteActionData Object Reference"))
  (for _array_element (`RogueliteSubsystem.GetAllAcquired` (subsystem `RogueliteSubsystem`))
    (if (`BlueprintSetLibrary.Set_Contains` (`self.PetAcquireActions`) _array_element)
      (bind _output_get (set `local.ActionToAcquire` _array_element))
      (for _ (range 1 (+ (`RogueliteSubsystem.GetActionStacks` (subsystem `RogueliteSubsystem`) _output_get) 1))
        (`self.OnActionAcquired` (`local.ActionToAcquire`))))))

(fn `Search Target`
  (locals (MinDistance :type "Float (double-precision)") (ClosestTarget :type "Actor Object Reference") (OwnerActor :type "Actor Object Reference"))
  (bind _owneractor (`local.OwnerActor`))
  (set `local.OwnerActor` (`self.GetOwner`))
  (set `local.MinDistance` 9999999999999.0)
  (set `local.ClosestTarget` null)
  (bind _outactors (`KismetSystemLibrary.SphereOverlapActors` (+ (`Actor.K2_GetActorLocation` _owneractor) (* (`Actor.GetActorForwardVector` _owneractor) (`self.SearchOffset`))) (`self.SearchRadius`) (`|MakeArray` "ObjectTypeQuery3" :!type "EObjectTypeQuery Enum") "/Script/Runner.EnemyBase"))
  (for _array_element _outactors
    (bind (_isclosest _newmindistance) (`self.IsClosestTarget` _array_element (`local.MinDistance`)))
    (if (and (`self.IsActorInFrontOfSource` _array_element (`local.OwnerActor`)) _isclosest)
      (set `local.MinDistance` _newmindistance)
      (set `local.ClosestTarget` _array_element)))
  (`/Engine/EditorBlueprintResources/StandardMacros.IsValid` (`local.ClosestTarget`)
    (:`Is Valid`
      (set `self.TargetActor` (`local.ClosestTarget`)))))

(fn `SetOwnerFollowLocationByIndex`
  (params (Index :type Integer) (OwnerFollowLocation :type "Vector Structure"))
  (bind _spawnedpets (`self.SpawnedPets`))
  (bind (_acquireaction _spawnedpet) (break `/Game/BP/Characters/Pet/ST_PetSpawnInfo` (`|GetArrayItem` _spawnedpets Index)))
  (if (`KismetArrayLibrary.Array_IsValidIndex` _spawnedpets Index)
    (`/Engine/EditorBlueprintResources/StandardMacros.IsValid` _spawnedpet
      (:`Is Valid`
        (`/Game/BP/Characters/Pet/BP_Pet.SetOwnerFollowLocation` _spawnedpet OwnerFollowLocation)))))

(fn `SetTargetToPets`
  (for _array_element (`self.SpawnedPets`)
    (bind (_acquireaction _spawnedpet) (break `/Game/BP/Characters/Pet/ST_PetSpawnInfo` _array_element))
    (`/Engine/EditorBlueprintResources/StandardMacros.IsValid` _spawnedpet
      (:`Is Valid`
        (set `/Game/BP/Characters/Pet/BP_Pet.TargetEnemyToChase` (`self.TargetActor`) _spawnedpet)))))

(fn `SpawnPetFromAction`
  (params (InAction :type "RogueliteActionData Object Reference"))
  (locals (PetAction :type "RogueliteActionData Object Reference") (OwnerCharacter :type "Character Object Reference") (SpawnedPet :type "/Game/BP/Characters/Pet/BP_Pet Object Reference") (SpawnTransform :type "Transform Structure"))
  (bind _returnvalue (`self.GetOwner`))
  (set `local.PetAction` InAction)
  (bind _ascharacter (cast `Character` (`self.GetOwner`)))
  (set `local.OwnerCharacter` _ascharacter)
  (`|ExecutionSequence`
    (:`then_0`
      (if (`self.bRemovedPet`)
        (set `local.SpawnTransform` (`self.LastRemovedPetTransform`))
        (else
          (set `local.SpawnTransform` (`KismetMathLibrary.MakeTransform` (`KismetMathLibrary.RandomPointInBoundingBox` (`Actor.K2_GetActorLocation` _returnvalue) (100.0 0.0 0.0)) (`Actor.K2_GetActorRotation` _returnvalue))))))
    (:`then_1`
      (bind _returnvalue_2 (`|SpawnActorFromClass` "/Game/BP/Characters/Pet/BP_Pet.BP_Pet_C" (`local.SpawnTransform`) "Undefined" "MultiplyWithRoot" null null))
      (bind _output_get (set `local.SpawnedPet` _returnvalue_2))
      (`/Game/BP/Characters/Pet/BP_Pet.InitPet` _output_get (`local.OwnerCharacter`) (`KismetMathLibrary.Conv_Int64ToInt` (`RogueliteActionData.GetValueAsInt` (`local.PetAction`) (struct :`TagName` "Pet.Stat.Level") 0)))
      (`KismetArrayLibrary.Array_Add` (`self.SpawnedPets`) (make `/Game/BP/Characters/Pet/ST_PetSpawnInfo` (`local.PetAction`) (`local.SpawnedPet`)))
      (`self.UpdatePetIndex`)
      (`self.Search Target`))))

(fn `UpdateOwnerFollowLocations`
  (locals (OwnerLocation :type "Vector Structure" :default (0.0 0.0 0.0)) (BackwardVector :type "Vector Structure") (NumPets :type Integer :default 0) (AngleStep :type "Float (double-precision)") (StartAngle :type "Float (double-precision)") (TargetAngle :type "Float (double-precision)") (TargetDirection :type "Vector Structure" :default (0.0 0.0 0.0)) (CurrentPetSpawnInfo :type "/Game/BP/Characters/Pet/ST_PetSpawnInfo Structure") (CurrentIndex :type Integer))
  (bind _returnvalue (`self.GetOwner`))
  (if (`KismetArrayLibrary.Array_IsEmpty` (`self.SpawnedPets`))
    (return)
    (else
      (set `local.OwnerLocation` (`Actor.K2_GetActorLocation` _returnvalue))
      (set `local.BackwardVector` (* (`Actor.GetActorForwardVector` _returnvalue) -1.0))
      (bind _output_get (set `local.NumPets` (`KismetArrayLibrary.Array_Length` (`self.SpawnedPets`))))
      (if (== _output_get 1)
        (`self.SetOwnerFollowLocationByIndex` 0 (+ (`local.OwnerLocation`) (* (`local.BackwardVector`) (`self.FollowLength`))))
        (return)
        (else
          (set `local.AngleStep` (/ 180.0 (`KismetMathLibrary.Conv_IntToDouble` (- (`local.NumPets`) 1))))
          (set `local.StartAngle` -90.0)
          (for (_ _array_index) (`self.SpawnedPets`)
            (set `local.CurrentIndex` _array_index)
            (set `local.TargetAngle` (+ (`local.StartAngle`) (* (`local.AngleStep`) (`local.CurrentIndex`))))
            (bind _output_get_2 (set `local.TargetDirection` (`KismetMathLibrary.Vector_Normal2D` (`KismetMathLibrary.RotateAngleAxis` (`local.BackwardVector`) (`local.TargetAngle`) (0.0 0.0 1.0)))))
            (`self.SetOwnerFollowLocationByIndex` (`local.CurrentIndex`) (+ (`local.OwnerLocation`) (* _output_get_2 (`self.FollowLength`))))))))))

(fn `UpdatePetIndex`
  (for (_array_element _array_index) (`self.SpawnedPets`)
    (bind (_acquireaction _spawnedpet) (break `/Game/BP/Characters/Pet/ST_PetSpawnInfo` _array_element))
    (`/Engine/EditorBlueprintResources/StandardMacros.IsValid` _spawnedpet
      (:`Is Valid`
        (`/Game/BP/Characters/Pet/BP_Pet.SetIndex` _spawnedpet _array_index)))))