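; Damage handler component that spawns floating damage feedback actors when damage is applied.
; OnDamageApplied checks the result's tags for Data.Critical to pick the damage type, then passes it and the amount to SpawnDamageWidget.
; If widget spawning is enabled and the actor class is valid, it pulls an actor from a pool at the owner's transform and initializes it with a fixed lifetime.
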(event `self.OnDamageApplied`
  (params (InDamageResult :type "DamageResult Structure (by ref)"))
  (bind (_damage _tags) (break `DamageResult` InDamageResult))
  (if (`BlueprintGameplayTagLibrary.HasTag` _tags (struct :`TagName` "Data.Critical"))
    (`self.SpawnDamageWidget` "NewEnumerator1" _damage)
    (else
      (`self.SpawnDamageWidget` "NewEnumerator0" _damage))))

(event `SpawnDamageWidget`
  (params (DamageType :type "/Game/BP/Combat/E_DamageType Enum" :default "NewEnumerator0") (DamageAmount :type "Float (double-precision)"))
  (bind _returnvalue (`self.GetOwner`))
  (if (`self.EnableSpawnWidget`)
    (bind _damageactorclass (`self.DamageActorClass`)
      (:`then`
        (bind _returnvalue_2 (`ObjectPoolBlueprintLibrary.SpawnFromPool` _damageactorclass (`KismetMathLibrary.MakeTransform` (`Actor.K2_GetActorLocation` _returnvalue) (`Actor.K2_GetActorRotation` _returnvalue)) "Undefined"))
        (`/Game/BP/Combat/BP_DamageWidgetActor.InitDamageActor` _returnvalue_2 DamageType DamageAmount 3.0))
      (:`else`))))