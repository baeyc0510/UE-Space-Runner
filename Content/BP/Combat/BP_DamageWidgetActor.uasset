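; BP_DamageWidgetActor is a pooled actor that shows a floating damage number through a widget component.
; InitDamageActor stores type, amount and lifetime, and pool activation defers display to the next tick.
; It then colors the rounded amount white for normal or orange for critical hits and plays the W_FloatingWidget animation.
; After the lifetime delay, it returns itself to the pool.
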(event `InitDamageActor`
  (params (DamageType :type "/Game/BP/Combat/E_DamageType Enum" :default "NewEnumerator0") (DamageAmount :type "Float (double-precision)") (DamageLifeTime :type "Float (double-precision)" :default 3.0))
  (set `self.DamageType` DamageType)
  (set `self.DamageAmount` DamageAmount)
  (set `self.DamageLifeTime` DamageLifeTime))

(event `PoolableInterface.OnPoolableActivate`
  (`KismetSystemLibrary.K2_SetTimerForNextTickDelegate` (delegate `OnNextTick`)))

(event `OnNextTick`
  (bind _asw_floating_widget (cast `/Game/BP/UI/W_FloatingWidget` (`WidgetComponent.GetWidget` (`self.WidgetComp`))))
  (set `self.WidgetInstance` _asw_floating_widget)
  (`|ExecutionSequence`
    (:`then_0`
      (switch `/Game/BP/Combat/E_DamageType` (`self.DamageType`)
        (:`NewEnumerator0`
          (set `self.DamageColor` (struct :`R` 1.0 :`G` 1.0 :`B` 1.0 :`A` 1.0)))
        (:`NewEnumerator1`
          (set `self.DamageColor` (struct :`R` 1.0 :`G` 0.448528 :`B` 0.026334 :`A` 1.0)))))
    (:`then_1`
      (`/Game/BP/UI/W_FloatingWidget.InitWidget` (`self.WidgetInstance`) (`KismetTextLibrary.Conv_Int64ToText` (`KismetMathLibrary.Round64` (`self.DamageAmount`))) (`self.DamageColor`))
      (`/Game/BP/UI/W_FloatingWidget.PlayFloatingAnimation` (`self.WidgetInstance`)))
    (:`then_2`
      (`KismetSystemLibrary.Delay` (`self.DamageLifeTime`))
      (`ObjectPoolBlueprintLibrary.ReturnToPool` null))))

(fn `UserConstructionScript`)