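; Manages an owner's stock of pooled BP_Missile projectiles for what the stat tag names the Sword ability, and fires them at a target.
; The maximum count follows the roguelite run-state stat, topping up missiles when it changes.
; New missiles spawn in rows and columns offset from the owner's transform.
; FireMissiles launches every unfired missile and notifies per shot; RemoveMissile frees capacity for recharging.
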(event `self.ReceiveBeginPlay`
  (set `self.MaxMissileCount` (`KismetMathLibrary.FTrunc` (`RogueliteBlueprintLibrary.GetRunStateValue` (struct :`TagName` "Stat.Ability.Sword.MaxCount"))))
  (add `RogueliteSubsystem.OnRunStateValueChanged` (subsystem `RogueliteSubsystem`) (delegate `OnRunStateValueChanged_Event`)))

(event `OnRunStateValueChanged_Event`
  (params (Key :type "GameplayTag Structure") (OldValue :type "Float (single-precision)") (NewValue :type "Float (single-precision)"))
  (if (`BlueprintGameplayTagLibrary.MatchesTag` Key (struct :`TagName` "Stat.Ability.Sword.MaxCount") true)
    (`self.ResizeMissiles` (`KismetMathLibrary.FTrunc` NewValue))))

(event `self.ReceiveTick`
  (params (DeltaSeconds :type "Float (single-precision)")))

(fn `FindEmptyMissileIndex`
  (returns (ReturnValue :type Integer))
  (locals (Indices :type "Set of Integer"))
  (return (`KismetArrayLibrary.Array_Length` (`self.SpawnedMissiles`))))

(fn `FireMissiles`
  (params (MissilePower :type "Float (double-precision)") (MissileSpeed :type "Float (double-precision)") (MissileMaxDistance :type "Float (double-precision)") (TargetActor :type "Actor Object Reference"))
  (`/Engine/EditorBlueprintResources/StandardMacros.IsValid` TargetActor
    (:`Is Valid`
      (for _array_element (`self.SpawnedMissiles`)
        (`/Engine/EditorBlueprintResources/StandardMacros.IsValid` _array_element
          (:`Is Valid`
            (if (not (`/Game/BP/Projectile/BP_Missile.IsFired` _array_element))
              (`/Game/BP/Projectile/BP_Missile.FireMissile` _array_element (`local.MissilePower`) (`local.MissileSpeed`) (`local.MissileMaxDistance`) (`local.TargetActor`))
              (`self.OnFiredMissiles`))))))))

(fn `GetMissileTransform`
  (params (InMissileIndex :type Integer))
  (returns (Transform :type "Transform Structure"))
  (locals (Offset :type "Float (double-precision)") (MissileRow :type Integer) (MissileColumn :type Integer :default 0))
  (bind _returnvalue (`self.GetOwner`))
  (set `local.MissileRow` (/ (+ (`local.InMissileIndex`) 1) (`self.MissileMaxColumn`)))
  (set `local.MissileColumn` (mod (`local.InMissileIndex`) (`self.MissileMaxColumn`)))
  (set `local.Offset` (- (`local.MissileColumn`) (/ (- (`self.MaxMissileCount`) 1) 2.0)))
  (return (`KismetMathLibrary.MakeTransform` (+ (`Actor.K2_GetActorLocation` _returnvalue) (* (`Actor.GetActorUpVector` _returnvalue) (`self.Height`)) (* (`Actor.GetActorRightVector` _returnvalue) (`local.Offset`) (`self.MissileSpacing`)) (* (`Actor.GetActorForwardVector` _returnvalue) (`self.MissileSpacing`) (`local.MissileRow`) -1.0)) (`Actor.K2_GetActorRotation` _returnvalue))))

(fn `HasAnyMissile`
  (returns (HasAnySword :type Boolean))
  (return (`KismetArrayLibrary.Array_IsNotEmpty` (`self.SpawnedMissiles`))))

(fn `IsFull`
  (returns (IsFull :type Boolean))
  (return (== (`KismetArrayLibrary.Array_Length` (`self.SpawnedMissiles`)) (`self.MaxMissileCount`))))

(fn `RechargeMissiles`
  (locals (CountToCharge :type Integer) (Added :type Boolean :default false))
  (bind _output_get (set `local.CountToCharge` (- (`self.MaxMissileCount`) (`KismetArrayLibrary.Array_Length` (`self.SpawnedMissiles`)))))
  (for _ (range 1 (+ _output_get 1))
    (`self.TryAddMissile`)))

(fn `RemoveMissile`
  (params (InMissile :type "/Game/BP/Projectile/BP_Missile Object Reference (by ref)"))
  (`KismetArrayLibrary.Array_RemoveItem` (`self.SpawnedMissiles`) InMissile))

(fn `ResizeMissiles`
  (params (Size :type Integer))
  (set `self.MaxMissileCount` Size)
  (`self.RechargeMissiles`))

(fn `TryAddMissile`
  (returns (Success :type Boolean))
  (bind _returnvalue (`self.FindEmptyMissileIndex`))
  (if (< (`KismetArrayLibrary.Array_Length` (`self.SpawnedMissiles`)) (`self.MaxMissileCount`))
    (if (>= _returnvalue 0)
      (bind _returnvalue_2 (`ObjectPoolBlueprintLibrary.SpawnFromPool` "/Game/BP/Projectile/BP_Missile.BP_Missile_C" (`self.GetMissileTransform` _returnvalue)))
      (`/Game/BP/Projectile/BP_Missile.InitMissile` _returnvalue_2 self (`self.GetOwner`) _returnvalue)
      (`KismetArrayLibrary.Array_Add` (`self.SpawnedMissiles`) _returnvalue_2)
      (return true)
      (else
        (return false)))))