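; Shop manager that handles stock, purchases and the currency balance for roguelite shop items.
; Stock loads from a save slot or the title game mode's DataTable; saving writes only item status, though loading also reads purchased actions.
; Currency mirrors the Roguelite subsystem's run-state value, updated through its change event.
; Purchases check stock and funds, deduct currency, decrement stock, record the action for stack counting, and broadcast changes.
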(event `self.ReceiveBeginPlay`
  (set `self.Currency` (`KismetMathLibrary.Conv_DoubleToInt64` (`RogueliteBlueprintLibrary.GetRunStateValue` (struct :`TagName` "GameState.Currency"))))
  (add `RogueliteSubsystem.OnRunStateValueChanged` (subsystem `RogueliteSubsystem`) (delegate `OnRunStateValueChanged_Event`))
  (`self.OnCurrenyChanged` (`self.Currency`)))

(event `OnRunStateValueChanged_Event`
  (params (Key :type "GameplayTag Structure") (OldValue :type "Float (single-precision)") (NewValue :type "Float (single-precision)"))
  (if (== Key (struct :`TagName` "GameState.Currency"))
    (bind _output_get (set `self.Currency` (`KismetMathLibrary.Conv_DoubleToInt64` NewValue)))
    (`self.OnCurrenyChanged` _output_get)))

(fn `CanPurchaseItem`
  (params (ItemIndex :type Integer))
  (returns (CanPurchase :type Boolean))
  (bind (_itemaction _sellcost _currentstack) (break `/Game/Data/Shop/ST_ShopItemStatus` (`|GetArrayItem` (`self.CurrentShopItems`) ItemIndex)))
  (return (and (> _currentstack 0) (`self.HasEnoughMoney` _sellcost))))

(fn `GetCurrentCurrency`
  (returns (Amount :type Integer64))
  (return (`self.Currency`)))

(fn `GetPurchasedActionStack`
  (params (InAction :type "RogueliteActionData Object Reference"))
  (returns (Stack :type Integer))
  (locals (StackCount :type Integer))
  (for _array_element (`self.PurchasedActions`)
    (if (== _array_element InAction)
      (`/Engine/EditorBlueprintResources/StandardMacros.IncrementInt` (`local.StackCount`))))
  (return (`local.StackCount`)))

(fn `HasEnoughMoney`
  (params (NeedAmount :type Integer64))
  (returns (bHasEnough :type Boolean))
  (return (<= NeedAmount (`self.Currency`))))

(fn `InitShopItems`
  (params (bTryLoad :type Boolean))
  (if bTryLoad
    (`self.LoadFromSaveData`)
    (else
      (`self.LoadFromDataTable`))))

(fn `LoadFromDataTable`
  (locals (ShopItemListTable :type "DataTable Object Reference"))
  (`KismetArrayLibrary.Array_Clear` (`self.CurrentShopItems`))
  (`KismetArrayLibrary.Array_Clear` (`self.PurchasedActions`))
  (bind _asbp_title_game_mode (cast `/Game/BP/GameFramework/Title/BP_TitleGameMode` (`GameplayStatics.GetGameMode`)))
  (bind _output_get (set `local.ShopItemListTable` (`/Game/BP/GameFramework/Title/BP_TitleGameMode.ShopItemDataTable` _asbp_title_game_mode)))
  (`/Engine/EditorBlueprintResources/StandardMacros.IsValid` _output_get
    (:`Is Valid`
      (bind _outrownames (`DataTableFunctionLibrary.GetDataTableRowNames` (`local.ShopItemListTable`)))
      (for _array_element _outrownames
        (bind _returnvalue (`|GetDataTableRow` (`local.ShopItemListTable`) _array_element)
          (:`then`
            (bind (_itemaction _sellcost _maxamount) (break `/Game/Data/Shop/ST_ShopItemInfo` _returnvalue))
            (`KismetArrayLibrary.Array_Add` (`self.CurrentShopItems`) (make `/Game/Data/Shop/ST_ShopItemStatus` _itemaction _sellcost _maxamount))))))))

(fn `LoadFromSaveData`
  (`KismetArrayLibrary.Array_Clear` (`self.CurrentShopItems`))
  (`KismetArrayLibrary.Array_Clear` (`self.PurchasedActions`))
  (bind _returnvalue (`GameplayStatics.DoesSaveGameExist` (`self.SaveSlotName`)))
  (if _returnvalue
    (bind _returnvalue_2 (`GameplayStatics.LoadGameFromSlot` (`self.SaveSlotName`)))
    (bind _asbp_shop_item_save_data (cast `/Game/Data/Shop/BP_ShopItemSaveData` _returnvalue_2))
    (set `self.CurrentShopItems` (`/Game/Data/Shop/BP_ShopItemSaveData.SavedShopItems` _asbp_shop_item_save_data))
    (set `self.PurchasedActions` (`/Game/Data/Shop/BP_ShopItemSaveData.PurchasedActions` _asbp_shop_item_save_data))
    (else
      (`self.LoadFromDataTable`))))

(fn `RemoveMoney`
  (params (Amount :type Integer64))
  (`RogueliteBlueprintLibrary.SetRunStateValue` (struct :`TagName` "GameState.Currency") (`KismetMathLibrary.Conv_Int64ToDouble` (`KismetMathLibrary.MaxInt64` (- (`self.Currency`) Amount)))))

(fn `SaveShopItems`
  (bind _returnvalue (`GameplayStatics.CreateSaveGameObject` "/Game/Data/Shop/BP_ShopItemSaveData.BP_ShopItemSaveData_C"))
  (set `/Game/Data/Shop/BP_ShopItemSaveData.SavedShopItems` (`self.CurrentShopItems`) _returnvalue)
  (`GameplayStatics.SaveGameToSlot` _returnvalue (`self.SaveSlotName`)))

(fn `TryPurchaseItem`
  (params (ItemIndex :type Integer))
  (locals (NewStack :type Integer) (TargetItem :type "/Game/Data/Shop/ST_ShopItemStatus Structure"))
  (bind _itemaction (break `/Game/Data/Shop/ST_ShopItemStatus` (`local.TargetItem`)))
  (bind (_itemaction_2 _sellcost _currentstack) (break `/Game/Data/Shop/ST_ShopItemStatus` (`local.TargetItem`)))
  (if (`self.CanPurchaseItem` ItemIndex)
    (set `local.TargetItem` (`|GetArrayItem` (`self.CurrentShopItems`) (`local.ItemIndex`)))
    (`|ExecutionSequence`
      (:`then_0`
        (`self.RemoveMoney` _sellcost)
        (bind _output_get (set `local.NewStack` (- _currentstack 1)))
        (setmembers `/Game/Data/Shop/ST_ShopItemStatus` :`StructRef` (`local.TargetItem`) :`CurrentStack` _output_get)
        (`KismetArrayLibrary.Array_Set` (`self.CurrentShopItems`) (`local.ItemIndex`) (`local.TargetItem`))
        (`self.OnShopItemChanged` (`local.ItemIndex`) (`local.TargetItem`)))
      (:`then_1`
        (`KismetArrayLibrary.Array_Add` (`self.PurchasedActions`) _itemaction)
        (`self.OnActionStackChanged` _itemaction (`self.GetPurchasedActionStack` _itemaction))))))