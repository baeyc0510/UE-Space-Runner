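; Pooled bullet projectile that flies straight forward and damages combat actors it touches.
; On pool activation it restarts its Niagara effect, sets velocity from the values given to InitBullet, then returns to the pool after max distance divided by speed.
; Capsule overlaps skip the owner and send CombatInterface targets a damage context carrying bullet power as base damage, then return the bullet to the pool.
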(event `PoolableInterface.OnPoolableActivate`
  (bind _projectilemovement (`self.ProjectileMovement`))
  (`NiagaraComponent.ReinitializeSystem` (`self.Niagara`))
  (set `ProjectileMovementComponent.InitialSpeed` (`self.BulletSpeed`) _projectilemovement)
  (set `ProjectileMovementComponent.MaxSpeed` (`self.BulletSpeed`) _projectilemovement)
  (set `MovementComponent.Velocity` (* (`self.GetActorForwardVector`) (`self.BulletSpeed`)) _projectilemovement)
  (`KismetSystemLibrary.Delay` (`KismetMathLibrary.SafeDivide` (`self.BulletMaxDistance`) (`self.BulletSpeed`)))
  (`ObjectPoolBlueprintLibrary.ReturnToPool` self))

(event `self.Capsule.OnComponentBeginOverlap`
  (params (OverlappedComponent :type "PrimitiveComponent Object Reference") (OtherActor :type "Actor Object Reference") (OtherComp :type "PrimitiveComponent Object Reference") (OtherBodyIndex :type Integer) (bFromSweep :type Boolean) (SweepResult :type "HitResult Structure (by ref)"))
  (`self.HandleHitOtherActor` OtherActor))

(fn `HandleHitOtherActor`
  (params (OtherActor :type "Actor Object Reference"))
  (locals (DamageContext :type "DamageContext Structure"))
  (if (!= OtherActor (`self.OwnerActor`))
    (if (and (`KismetSystemLibrary.DoesImplementInterface` (`local.OtherActor`) "/Script/Runner.CombatInterface") (`KismetSystemLibrary.IsValid` (`self.OwnerActor`)))
      (set `local.DamageContext` (`CombatBlueprintLibrary.CreateDamageContext` self (`local.OtherActor`) (`self.OwnerActor`)))
      (`BlueprintMapLibrary.Map_Add` (`.SourceValues` (break `DamageContext` (`local.DamageContext`))) (struct :`TagName` "Data.BaseDamage") (`self.BulletPower`))
      (message `CombatInterface.ApplyDamage` (`local.OtherActor`) (`local.DamageContext`))
      (`ObjectPoolBlueprintLibrary.ReturnToPool` self))))

(fn `InitBullet`
  (params (OwnerActor :type "Actor Object Reference") (BulletPower :type "Float (double-precision)") (BulletSpeed :type "Float (double-precision)") (BulletMaxDistance :type "Float (double-precision)"))
  (set `self.OwnerActor` OwnerActor)
  (set `self.BulletPower` BulletPower)
  (set `self.BulletSpeed` BulletSpeed)
  (set `self.BulletMaxDistance` BulletMaxDistance))

(fn `UserConstructionScript`)