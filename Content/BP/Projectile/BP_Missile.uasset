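; BP_Missile is a pooled homing projectile that waits in a missile manager's formation until fired at a target.
; While unfired it has collision off and interpolates toward its indexed slot transform.
; FireMissile enables homing and overlap collision, then leaves the manager; Tick eases rotation toward velocity.
; Any overlap returns it to the pool, first damaging CombatInterface actors through a DamageContext, as does exceeding range or lifetime.
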(event `PoolableInterface.OnPoolableActivate`
  (`PrimitiveComponent.SetCollisionEnabled` (`self.Capsule`) "NoCollision")
  (set `self.IsFired` false))

(event `self.ReceiveTick`
  (params (DeltaSeconds :type "Float (single-precision)"))
  (if (`self.IsFired`)
    ;[1 1 1] 디스폰(최대거리,시간)
    (if (or (> (`KismetMathLibrary.Vector_Distance` (`self.FiredLocation`) (`self.K2_GetActorLocation`)) (`self.MaxDistance`)) (> (- (`KismetSystemLibrary.GetGameTimeInSeconds`) (`self.FiredTime`)) 5.0))
      (`ObjectPoolBlueprintLibrary.ReturnToPool` null)
      (else
        ;[1 1 1] 플레이어 따라가기
        (if (not (`KismetMathLibrary.Vector_IsNearlyZero` (`MovementComponent.Velocity` (`self.ProjectileMovement`))))
          (`self.K2_SetActorRotation` (`KismetMathLibrary.RInterpTo` (`self.K2_GetActorRotation`) (`KismetMathLibrary.MakeRotFromX` (`MovementComponent.Velocity` (`self.ProjectileMovement`))) (`GameplayStatics.GetWorldDeltaSeconds`) 9.0)))))
    (else
      ;[1 1 1] 유도 모드
      (bind _owningmissilemanager (`self.OwningMissileManager`)
        (:`then`
          (`self.K2_SetActorLocationAndRotation` (`KismetMathLibrary.VInterpTo` (`self.K2_GetActorLocation`) (.location (`/Game/BP/Combat/BP_MissileManager.GetMissileTransform` _owningmissilemanager (`self.MissileIndex`))) (`GameplayStatics.GetWorldDeltaSeconds`) 9.0) (`KismetMathLibrary.RInterpTo` (`self.K2_GetActorRotation`) (.rotation (`/Game/BP/Combat/BP_MissileManager.GetMissileTransform` _owningmissilemanager (`self.MissileIndex`))) (`GameplayStatics.GetWorldDeltaSeconds`) 9.0)))
        (:`else`)))))

(event `self.Capsule.OnComponentBeginOverlap`
  (params (OverlappedComponent :type "PrimitiveComponent Object Reference") (OtherActor :type "Actor Object Reference") (OtherComp :type "PrimitiveComponent Object Reference") (OtherBodyIndex :type Integer) (bFromSweep :type Boolean) (SweepResult :type "HitResult Structure (by ref)"))
  (`self.HandleHitOtherActor` OtherActor))

(fn `FireMissile`
  (params (MissilePower :type "Float (double-precision)") (MissileSpeed :type "Float (double-precision)") (MaxDistance :type "Float (double-precision)") (TargetActor :type "Actor Object Reference"))
  (bind _targetactor (`local.TargetActor`))
  (`|ExecutionSequence`
    (:`then_0`
      (set `self.MissilePower` MissilePower)
      (set `self.MissileSpeed` MissileSpeed)
      (set `self.MaxDistance` MaxDistance)
      (set `self.IsFired` true)
      (set `self.FiredLocation` (`self.K2_GetActorLocation`))
      (set `self.FiredTime` (`KismetSystemLibrary.GetGameTimeInSeconds`))
      (`local.TargetActor`
        (:`then`
          ;[1 1 1] TurnOnHommingMode
          (set `ProjectileMovementComponent.MaxSpeed` (`self.MissileSpeed`) (`self.ProjectileMovement`))
          (set `ProjectileMovementComponent.bIsHomingProjectile` true (`self.ProjectileMovement`))
          (set `ProjectileMovementComponent.HomingTargetComponent` (`Actor.RootComponent` (`local.TargetActor`)) (`self.ProjectileMovement`))
          (set `MovementComponent.Velocity` (* (`KismetMathLibrary.Normal` (- (+ (`self.K2_GetActorLocation` _targetactor) (* (`self.GetActorUpVector` _targetactor) 100.0)) (`self.K2_GetActorLocation`))) (`self.MissileSpeed`)) (`self.ProjectileMovement`)))
        (:`else`
          (`ObjectPoolBlueprintLibrary.ReturnToPool` null))))
    (:`then_1`
      (bind _capsule (`self.Capsule`)
        (:`then`
          (`PrimitiveComponent.SetCollisionEnabled` _capsule "QueryOnly"))
        (:`else`)))
    (:`then_2`
      (bind _owningmissilemanager (`self.OwningMissileManager`)
        (:`then`
          (`/Game/BP/Combat/BP_MissileManager.RemoveMissile` _owningmissilemanager self))
        (:`else`)))))

(fn `HandleHitOtherActor`
  (params (OtherActor :type "Actor Object Reference"))
  (locals (DamageContext :type "DamageContext Structure"))
  (if (and (`KismetSystemLibrary.DoesImplementInterface` (`local.OtherActor`) "/Script/Runner.CombatInterface") (`KismetSystemLibrary.IsValid` (`self.OwnerActor`)))
    (set `local.DamageContext` (`CombatBlueprintLibrary.CreateDamageContext` self (`local.OtherActor`) (`self.OwnerActor`)))
    (`BlueprintMapLibrary.Map_Add` (`.SourceValues` (break `DamageContext` (`local.DamageContext`))) (struct :`TagName` "Data.BaseDamage") (`self.MissilePower`))
    (message `CombatInterface.ApplyDamage` (`local.OtherActor`) (`local.DamageContext`))
    (`ObjectPoolBlueprintLibrary.ReturnToPool` null)
    (else
      (`ObjectPoolBlueprintLibrary.ReturnToPool` null))))

(fn `InitMissile`
  (params (MissileManager :type "/Game/BP/Combat/BP_MissileManager Object Reference") (OwnerActor :type "Actor Object Reference") (MissileIndex :type Integer))
  (set `self.OwningMissileManager` MissileManager)
  (set `self.OwnerActor` OwnerActor)
  (set `self.MissileIndex` MissileIndex)
  (set `self.IsFired` false))

(fn `UserConstructionScript`)