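; BP_RewardDoor is a reward door actor that displays the name of the reward action assigned to it.
; InitDoor stores the RewardAction and refreshes the label, which is also initialized on BeginPlay.
; InitWidget casts the widget component's widget to W_Text, then fills it with the BP_RunnerActionData formatted display name in white.
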(event `InitDoor`
  (params (RewardAction :type "RogueliteActionData Object Reference"))
  (set `self.RewardAction` RewardAction)
  (`self.InitWidget`))

(event `self.ReceiveBeginPlay`
  (`self.InitWidget`))

(fn `InitWidget`
  (bind _asw_text (cast `/Game/BP/UI/W_Text` (`WidgetComponent.GetWidget` (`self.WidgetComponent`))))
  (bind _output_get (set `self.TextWidget` _asw_text))
  (`/Engine/EditorBlueprintResources/StandardMacros.IsValid` _output_get
    (:`Is Valid`
      (bind _asbp_runner_action_data (cast `/Game/Data/RogueliteActions/BP_RunnerActionData` (`self.RewardAction`)))
      (`/Game/BP/UI/W_Text.SetContent` (`self.TextWidget`) (`/Game/Data/RogueliteActions/BP_RunnerActionData.GetFormattedDisplayName` _asbp_runner_action_data) (struct :`R` 1.0 :`G` 1.0 :`B` 1.0 :`A` 1.0)))))

(fn `UserConstructionScript`)