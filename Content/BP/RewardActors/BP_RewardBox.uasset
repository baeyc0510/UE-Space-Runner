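; BP_RewardBox is a pickup actor that grants a reward to the player who overlaps it.
; On BeginPlay it writes the formatted display name from its RewardAction, cast to BP_RunnerActionData, into a W_Text widget component and sets a short lifespan as a safety fallback.
; When BP_PlayerCharacter overlaps the Box, it passes RewardAction to GiveReward and destroys itself.
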(event `self.ReceiveBeginPlay`
  (bind _asw_text (cast `/Game/BP/UI/W_Text` (`WidgetComponent.GetWidget` (`self.WidgetComponent`))))
  (bind _output_get (set `self.TextWidget` _asw_text))
  (`/Engine/EditorBlueprintResources/StandardMacros.IsValid` _output_get
    (:`Is Valid`
      (bind _asbp_runner_action_data (cast `/Game/Data/RogueliteActions/BP_RunnerActionData` (`self.RewardAction`)))
      (`/Game/BP/UI/W_Text.SetContent` (`self.TextWidget`) (`/Game/Data/RogueliteActions/BP_RunnerActionData.GetFormattedDisplayName` _asbp_runner_action_data) (struct :`R` 1.0 :`G` 1.0 :`B` 1.0 :`A` 1.0))
      ;[1 1 1] 안전 코드
      (`self.SetLifeSpan` 5.0))))

(event `self.Box.OnComponentBeginOverlap`
  (params (OverlappedComponent :type "PrimitiveComponent Object Reference") (OtherActor :type "Actor Object Reference") (OtherComp :type "PrimitiveComponent Object Reference") (OtherBodyIndex :type Integer) (bFromSweep :type Boolean) (SweepResult :type "HitResult Structure (by ref)"))
  (bind _asbp_player_character (cast `/Game/BP/Characters/Player/BP_PlayerCharacter` OtherActor))
  (`/Game/BP/Characters/Player/BP_PlayerCharacter.GiveReward` _asbp_player_character (`self.RewardAction`))
  (`self.K2_DestroyActor`))

(fn `UserConstructionScript`)