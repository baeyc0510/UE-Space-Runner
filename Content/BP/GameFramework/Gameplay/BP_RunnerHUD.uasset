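; HUD Blueprint for the runner game that owns the W_HUD widget and relays gameplay updates to it.
; On BeginPlay it creates the widget, sets up the progress bar from the mid-boss count per stage and replays already acquired roguelite action stacks.
; It then binds to the roguelite subsystem for later stack changes.
; Events for progress, score and progress bar setup forward to the widget behind validity checks.
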(event `self.ReceiveBeginPlay`
  (bind _returnvalue (`|CreateWidget` "/Game/BP/UI/HUD/W_HUD.W_HUD_C" (`self.GetOwningPlayerController`)))
  (bind _output_get (set `self.HUDWidget` _returnvalue))
  (`UserWidget.AddToViewport` _output_get 0)
  (`/Game/BP/UI/HUD/W_HUD.InitProgressBar` _output_get (`self.Num Mid Boss Per Stage`))
  (for _array_element (`RogueliteBlueprintLibrary.GetAllAcquired`)
    (`self.OnActionStackChanged` _array_element (`RogueliteBlueprintLibrary.GetActionStacks` _array_element)))
  (add `RogueliteSubsystem.OnStackChanged` (subsystem `RogueliteSubsystem`) (delegate `CustomEvent`)))

(event `UpdateProgress`
  (params (InPercent :type "Float (single-precision)"))
  (bind _hudwidget (`self.HUDWidget`)
    (:`then`
      (`/Game/BP/UI/HUD/W_HUD.UpdateProgressBar` _hudwidget InPercent))
    (:`else`)))

(event `CustomEvent`
  (params (Action :type "RogueliteActionData Object Reference") (OldStacks :type Integer) (NewStacks :type Integer))
  (`self.OnActionStackChanged` Action NewStacks))

(event `OnActionStackChanged`
  (params (InAction :type "RogueliteActionData Object Reference") (NewStack :type Integer))
  (bind _hudwidget (`self.HUDWidget`)
    (:`then`
      (`/Game/BP/UI/HUD/W_HUD.OnActionStackChanged` _hudwidget InAction NewStack))
    (:`else`)))

(event `UpdateScore`
  (params (NewScore :type Integer))
  (bind _hudwidget (`self.HUDWidget`)
    (:`then`
      (`/Game/BP/UI/HUD/W_HUD.UpdateScore` _hudwidget NewScore))
    (:`else`)))

(event `InitProgressBar`
  (params (NumMidBossPerStage :type Integer))
  (set `self.Num Mid Boss Per Stage` NumMidBossPerStage)
  (bind _hudwidget (`self.HUDWidget`)
    (:`then`
      (`/Game/BP/UI/HUD/W_HUD.InitProgressBar` _hudwidget NumMidBossPerStage))
    (:`else`)))

(fn `UserConstructionScript`)