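; Runner game state that tracks the score and the player's progress along the X axis toward each main boss.
; InitProgress derives the main boss distance from tile size and round interval, then sets up the HUD progress bar from the boss interval ratio.
; UpdateProgress wraps offset-adjusted distance from start with modulo into a repeating stage fraction.
; Progress and score changes are broadcast through event dispatchers.
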(fn `AddScore`
  (params (Delta :type Integer))
  (bind _output_get (set `self.CurrentScore` (+ (`self.CurrentScore`) Delta)))
  (`self.OnUpdateScore` _output_get))

(fn `InitProgress`
  (params (TileSizeX :type "Float (double-precision)") (MidBossRoundInterval :type Integer) (MainBossRoundInterval :type Integer))
  (bind _returnvalue (`GameplayStatics.GetPlayerController` 0))
  (set `self.TileSizeX` TileSizeX)
  (set `self.MidBossRoundInterval` MidBossRoundInterval)
  (set `self.MainBossRoundInterval` MainBossRoundInterval)
  (set `self.DistanceToMainBoss` (* (`self.TileSizeX`) (`self.MainBossRoundInterval`)))
  (`/Engine/EditorBlueprintResources/StandardMacros.IsValid` _returnvalue
    (:`Is Valid`
      (bind _asbp_runner_hud (cast `/Game/BP/GameFramework/Gameplay/BP_RunnerHUD` (`PlayerController.GetHUD` _returnvalue)))
      (`/Game/BP/GameFramework/Gameplay/BP_RunnerHUD.InitProgressBar` _asbp_runner_hud (- (/ (`self.MainBossRoundInterval`) (`self.MidBossRoundInterval`)) 1)))))

(fn `UpdateProgress`
  (params (StartPosX :type "Float (double-precision)") (CuurentPosX :type "Float (double-precision)"))
  (locals (DistanceFromStart :type "Float (double-precision)"))
  (set `self.StartPosX` StartPosX)
  (set `self.CuurentPosX` CuurentPosX)
  (if (> (`self.DistanceToMainBoss`) 0.1)
    (bind _output_get (set `local.DistanceFromStart` (- (`self.CuurentPosX`) (`self.StartPosX`))))
    (bind _output_get_2 (set `self.CurrentStageProgress` (/ (mod (- _output_get (`self.StartOffset`)) (`self.DistanceToMainBoss`)) (`self.DistanceToMainBoss`))))
    (`self.OnUpdateProgress` _output_get_2)))

(fn `UserConstructionScript`)