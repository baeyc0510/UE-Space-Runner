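; BP_RunnerPlayerController is the runner game's player controller that relays stage progress and score from the game state to the HUD.
; On BeginPlay it caches BP_RunnerHUD and BP_RunnerGameState, subscribes to the game state's progress and score update dispatchers, and pushes the current values to the HUD.
; Later updates arrive through the bound events, which forward each new value to the HUD after a validity check.
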(event `self.ReceiveBeginPlay`
  (`|ExecutionSequence`
    (:`then_0`
      (bind _asbp_runner_hud (cast `/Game/BP/GameFramework/Gameplay/BP_RunnerHUD` (`self.GetHUD`)))
      (set `self.RunnerHUD` _asbp_runner_hud))
    (:`then_1`
      (bind _asbp_runner_game_state (cast `/Game/BP/GameFramework/Gameplay/BP_RunnerGameState` (`GameplayStatics.GetGameState`)))
      (bind _output_get (set `self.RunnerGameState` _asbp_runner_game_state))
      (`|ExecutionSequence`
        (:`then_0`
          (add `/Game/BP/GameFramework/Gameplay/BP_RunnerGameState.OnUpdateProgress` _output_get (delegate `OnUpdateProgress_Event`))
          (bind _runnerhud (`self.RunnerHUD`)
            (:`then`
              (`/Game/BP/GameFramework/Gameplay/BP_RunnerHUD.UpdateProgress` _runnerhud (`/Game/BP/GameFramework/Gameplay/BP_RunnerGameState.CurrentStageProgress` (`self.RunnerGameState`))))
            (:`else`)))
        (:`then_1`
          (add `/Game/BP/GameFramework/Gameplay/BP_RunnerGameState.OnUpdateScore` _output_get (delegate `OnUpdateScore_Event`))
          (bind _runnerhud_2 (`self.RunnerHUD`)
            (:`then`
              (`/Game/BP/GameFramework/Gameplay/BP_RunnerHUD.UpdateScore` _runnerhud_2 (`/Game/BP/GameFramework/Gameplay/BP_RunnerGameState.CurrentScore` (`self.RunnerGameState`))))
            (:`else`)))))))

(event `OnUpdateProgress_Event`
  (params (CurrentProgress :type "Float (double-precision)"))
  (bind _runnerhud (`self.RunnerHUD`)
    (:`then`
      (`/Game/BP/GameFramework/Gameplay/BP_RunnerHUD.UpdateProgress` _runnerhud CurrentProgress))
    (:`else`)))

(event `OnUpdateScore_Event`
  (params (CurrentScore :type Integer))
  (bind _runnerhud (`self.RunnerHUD`)
    (:`then`
      (`/Game/BP/GameFramework/Gameplay/BP_RunnerHUD.UpdateScore` _runnerhud CurrentScore))
    (:`else`)))

(fn `UserConstructionScript`)