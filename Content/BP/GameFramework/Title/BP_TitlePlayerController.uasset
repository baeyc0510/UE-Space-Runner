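; Player controller for the title screen, showing the mouse cursor and handling the start-play and shop actions.
; Starting play loads and registers roguelite subsystem actions, has BP_TitleGameState acquire purchased ones, then opens L_PlayMap.
; Opening the shop creates or reuses a cached W_Shop widget, initialized with the game state's ShopManager and given input focus.
; The exit handler is an empty stub.
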(event `self.ReceiveBeginPlay`
  (set `self.bShowMouseCursor` true)
  (`WidgetBlueprintLibrary.SetInputMode_GameAndUIEx` self null))

(fn `OnExit`)

(fn `OnOpenShop`
  (locals (ShopManager :type "/Game/BP/Shop/BP_ShopManager Object Reference"))
  (bind _asbp_title_game_state (cast `/Game/BP/GameFramework/Title/BP_TitleGameState` (`GameplayStatics.GetGameState`)))
  (set `local.ShopManager` (`/Game/BP/GameFramework/Title/BP_TitleGameState.ShopManager` _asbp_title_game_state))
  (`|ExecutionSequence`
    (:`then_0`
      (`/Engine/EditorBlueprintResources/StandardMacros.IsValid` (`self.ShopWidgetInstance`)
        (:`Is Valid`
          (if (`Widget.IsInViewport` (`self.ShopWidgetInstance`))
            (`Widget.SetVisibility` (`self.ShopWidgetInstance`) "Visible")
            (`WidgetBlueprintLibrary.SetInputMode_GameAndUIEx` self (`self.ShopWidgetInstance`) "DoNotLock" false)
            (return)))
        (:`Is Not Valid`
          (bind _returnvalue (`|CreateWidget` "/Game/BP/UI/Shop/W_Shop.W_Shop_C" self))
          (set `self.ShopWidgetInstance` _returnvalue))))
    (:`then_1`
      (`/Game/BP/UI/Shop/W_Shop.Init Shop` (`self.ShopWidgetInstance`) (`local.ShopManager`))
      (`UserWidget.AddToViewport` (`self.ShopWidgetInstance`) 0)
      (`WidgetBlueprintLibrary.SetInputMode_GameAndUIEx` self (`self.ShopWidgetInstance`) "DoNotLock" false))))

(fn `OnStartPlay`
  (`|ExecutionSequence`
    (:`then_0`
      (`RogueliteSubsystem.LoadAndRegisterActions` (subsystem `RogueliteSubsystem`) "RogueliteActionData")
      (bind _asbp_title_game_state (cast `/Game/BP/GameFramework/Title/BP_TitleGameState` (`GameplayStatics.GetGameState`)))
      (`/Game/BP/GameFramework/Title/BP_TitleGameState.AcquirePurchasedActions` _asbp_title_game_state))
    (:`then_1`
      (`GameplayStatics.OpenLevelBySoftObjectPtr` "/Game/Maps/L_PlayMap.L_PlayMap"))))

(fn `UserConstructionScript`)