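; BP_TitleGameState is the game state for the title stage, managing a roguelite shop through its ShopManager.
; On BeginPlay it grants starting currency when save data is disabled, then initializes the shop items.
; Helper functions save shop items only when save data is enabled and queue each purchased action as a single-stack pending action in the roguelite subsystem.
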(event `self.ReceiveBeginPlay`
  (`|ExecutionSequence`
    (:`then_0`
      (if (not (`self.bUseSaveData`))
        (`RogueliteBlueprintLibrary.AddRunStateValue` (struct :`TagName` "GameState.Currency") 300.0)))
    (:`then_1`
      (`self.InitShopItems`))))

(fn `AcquirePurchasedActions`
  (for _array_element (`/Game/BP/Shop/BP_ShopManager.PurchasedActions` (`self.ShopManager`))
    (`RogueliteSubsystem.AddPendingAction` (subsystem `RogueliteSubsystem`) _array_element 1)))

(fn `InitShopItems`
  (`/Game/BP/Shop/BP_ShopManager.InitShopItems` (`self.ShopManager`) (`self.bUseSaveData`)))

(fn `SaveShopItems`
  (if (`self.bUseSaveData`)
    (`/Game/BP/Shop/BP_ShopManager.SaveShopItems` (`self.ShopManager`))))

(fn `UserConstructionScript`)